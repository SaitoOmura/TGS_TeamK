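; Enemy fan-shot emitter that spawns a spread of BP_Enemy_Bullet actors as soon as it begins play, then expires via a lifespan.
; FireFanBullet spaces BulletCount bullets evenly across SpreadAngle, centred on its own yaw, or fires one straight bullet when the count is below one.
; A count of exactly one still takes the fan path, dividing by zero.
; It also caches a BP_AdsorptionArea reference that is otherwise unused here.
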(event Custom|FireFanBullet
  (bind _returnvalue (Transformation|GetActorTransform))
  (if (>= (Variables|Default|GetBulletCount) 1)
    (Variables|Default|SetAngleStep (/ (Variables|Default|GetSpreadAngle) (- (Variables|Default|GetBulletCount) 1)))
    (Variables|Default|SetStartAngle (* (/ (Variables|Default|GetSpreadAngle) 2.0) -1.0))
    (for _index (range 0 (Math|Float|Truncate (- (Variables|Default|GetBulletCount) 1)))
      (Game|SpawnActorfromClass "/Game/Enemy/Blueprints/BP_Enemy_Bullet.BP_Enemy_Bullet_C" (Math|Transform|MakeTransform (.location _returnvalue) (Math|Rotator|MakeRotator (.roll (.rotation _returnvalue)) (.pitch (.rotation _returnvalue)) (+ (.yaw (.rotation _returnvalue)) (+ (Variables|Default|GetStartAngle) (* (Math|Conversions|ToFloat(Integer) _index) (Variables|Default|GetAngleStep))))) (.scale _returnvalue)) "Undefined" 0 0))
    (else
      (Game|SpawnActorfromClass "/Game/Enemy/Blueprints/BP_Enemy_Bullet.BP_Enemy_Bullet_C" (Transformation|GetActorTransform) "Undefined" 0 0))))

(event EventBeginPlay
  (bind _returnvalue (Actor|GetActorOfClass "/Game/ThirdPerson/Blueprints/BP_AdsorptionArea.BP_AdsorptionArea_C"))
  (Variables|Default|SetAdsorptionArea _returnvalue)
  (Actor|SetLifeSpan 1e+01)
  (CallFunction|FireFanBullet))

(event Collision|EventActorBeginOverlap
  (params (OtherActor :type Actor%20Object%20Reference)))

(event EventTick
  (params (DeltaSeconds :type Float%20%28single-precision%29)))

(fn ConstructionScript)