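; Barrier (baria) actor for the boss that follows BP_Boss_Enemy and absorbs BP_Burst hits until its durability runs out.
; It finds the boss on BeginPlay and snaps to its location every Tick.
; Each burst overlap decrements Taikyuuti, adds a Niagara component and hides the sphere.
; After a one-second delay the effect deactivates, and at zero durability it clears Isbaria and destroys itself.
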(event OnComponentBeginOverlap(baria)
  (params (OverlappedComponent :type Primitive%20Component%20Object%20Reference) (OtherActor :type Actor%20Object%20Reference) (OtherComp :type Primitive%20Component%20Object%20Reference) (OtherBodyIndex :type Integer) (bFromSweep :type Boolean) (SweepResult :type Hit%20Result%20Structure%20%28by%20ref%29))
  (Utilities|Casting|CastToBP_Burst OtherActor)
  (Math|Integer|DecrementInt (Variables|Default|Gettaikyuuti)
    (:%20%20
      (bind _returnvalue (AddComponent|AddNiagaraComponent true (Math|Transform|MakeTransform (+ (.location (Transformation|GetActorTransform)) "0.000000,0.000000,500.000000") "180.000000,0.000000,0.000000" "100.000000,100.000000,100.000000")))
      (Rendering|SetVisibility (Variables|Default|GetSphere) false false)
      (Utilities|FlowControl|Delay 1.0)
      (Components|Activation|Deactivate _returnvalue)
      (if (< (Variables|Default|Gettaikyuuti) 1)
        (Variables|Default|Setisbaria false)
        (Actor|DestroyActor)))))

(event Custom|CustomEvent
  (params (OverlappedComponent :type Primitive%20Component%20Object%20Reference) (OtherActor :type Actor%20Object%20Reference) (OtherComp :type Primitive%20Component%20Object%20Reference) (OtherBodyIndex :type Integer) (bFromSweep :type Boolean) (SweepResult :type Hit%20Result%20Structure%20%28by%20ref%29)))

(event EventBeginPlay
  (bind _returnvalue (Actor|GetActorOfClass "/Game/Enemy/Blueprints/BP_Boss_Enemy.BP_Boss_Enemy_C"))
  (Variables|Default|SetNewVar_0 _returnvalue))

(event Collision|EventActorBeginOverlap
  (params (OtherActor :type Actor%20Object%20Reference)))

(event EventTick
  (params (DeltaSeconds :type Float%20%28single-precision%29))
  (bind _newvar_0 (Variables|Default|GetNewVar_0))
  (Utilities|IsValid _newvar_0
    (:Is%20Valid
      (Transformation|SetActorLocation (Transformation|GetActorLocation _newvar_0) false false))))

(fn ConstructionScript)