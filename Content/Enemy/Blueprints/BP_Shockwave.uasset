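; Enemy shockwave actor that expands from a timeline on BeginPlay and destroys itself when the timeline finishes.
; The timeline scales a flattened Cylinder and Niagara effect horizontally, and a Capsule uniformly on all axes.
; Player overlap with the Cylinder deals damage unless an earlier Capsule overlap has set a flag, which is never cleared.
; Debug prints report the spawn location and overlap outcomes.
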(event OnComponentBeginOverlap(Capsule)
  (params (OverlappedComponent :type Primitive%20Component%20Object%20Reference) (OtherActor :type Actor%20Object%20Reference) (OtherComp :type Primitive%20Component%20Object%20Reference) (OtherBodyIndex :type Integer) (bFromSweep :type Boolean) (SweepResult :type Hit%20Result%20Structure%20%28by%20ref%29))
  (if (== (Game|Player|GetPlayerPawn 0) OtherActor)
    (Variables|Default|SetNewVar true)
    (Development|PrintString "Hello" true true "(R=0.622206,G=0.000000,B=1.000000,A=1.000000)")))

(event OnComponentBeginOverlap(Cylinder)
  (params (OverlappedComponent :type Primitive%20Component%20Object%20Reference) (OtherActor :type Actor%20Object%20Reference) (OtherComp :type Primitive%20Component%20Object%20Reference) (OtherBodyIndex :type Integer) (bFromSweep :type Boolean) (SweepResult :type Hit%20Result%20Structure%20%28by%20ref%29))
  (bind _returnvalue (Game|Player|GetPlayerPawn 0))
  (if (== _returnvalue OtherActor)
    (if (Variables|Default|GetNewVar)
      (Development|PrintString "Hello" true true "(R=0.000000,G=1.000000,B=0.197368,A=1.000000)")
      (else
        (Game|Damage|ApplyDamage _returnvalue 3e+01 0 0)
        (Development|PrintString "12345679" true true "(R=1.000000,G=0.057939,B=0.000000,A=1.000000)")))))

(event EventBeginPlay
  (Development|PrintString (Utilities|String|ToString(Vector) (Transformation|GetActorLocation)))
  (bind _新規track_0 (Timeline|タイムライン Play)
    (:Update
      (Transformation|SetWorldScale3D (Variables|Default|GetCylinder) (Math|Vector|MakeVector _新規track_0 _新規track_0 0.01))
      (Transformation|SetWorldScale3D (Variables|Default|GetCapsule) (Math|Vector|MakeVector _新規track_0 _新規track_0 _新規track_0)))
    (:Finished
      (Actor|DestroyActor))))

(event Collision|EventActorBeginOverlap
  (params (OtherActor :type Actor%20Object%20Reference)))

(event EventTick
  (params (DeltaSeconds :type Float%20%28single-precision%29)))

(fn ConstructionScript)