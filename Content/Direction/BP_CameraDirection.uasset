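; Level-intro camera actor that plays a short opening sequence, then hands the view over to gameplay.
; On BeginPlay it finds the current level in its Levelname array and picks a sequence by index: a simple hold, or timed MoveComponentTo camera moves for the second entry.
; All sequences end by blending to an actor tagged "main", destroying this actor and setting Start on BP_MyGameState.
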(event EventBeginPlay
  (bind _cameracomponent (Variables|CameraActor|GetCameraComponent))
  (bind _returnvalue (Game|GetCurrentLevelName true))
  (for (_array_element _array_index) (Variables|Default|Getlevelname)
    (if (Utilities|Enum|Equal(Enum) _array_element _returnvalue)
      (switch int _array_index
        (:0
          (Utilities|FlowControl|Delay 4.0 :!label _label))
        (:1
          (Utilities|FlowControl|Delay 1.0)
          (Components|MoveComponentTo _cameracomponent "600.000000,800.000000,700.000000" "0.000000,-90.000000,0.000000" false false 0.5 false)
          (Utilities|FlowControl|Delay 2.0)
          (Components|MoveComponentTo _cameracomponent "600.000000,1000.000000,300.000000" "0.000000,-90.000000,0.000000" false false 0.5 false)
          (Utilities|FlowControl|Delay 2.0))
        (:2
          (goto _label)))
      (bind _outactors (Actor|GetAllActorswithTag "main"))
      (for _array_element_2 _outactors
        (Variables|Default|SetArray%20Element _array_element_2))
      (Game|Player|SetViewTargetwithBlend (Game|GetPlayerController 0) (Variables|Default|GetArray%20Element) 1.0 "VTBlend_Linear" 0.0 false)
      (Utilities|FlowControl|Delay 0.2)
      (Actor|DestroyActor)
      (Variables|/Game/ThirdPerson/Blueprints/BP_MyGameState.BP_MyGameState_C|Setstart (.AsBP%20My%20Game%20State (Utilities|Casting|CastToBP_MyGameState (Game|GetGameState))) true))))

(event Collision|EventActorBeginOverlap
  (params (OtherActor :type Actor%20Object%20Reference)))

(event EventTick
  (params (DeltaSeconds :type Float%20%28single-precision%29)))

(fn ConstructionScript)